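; Gobang (five-in-a-row) match controller that resets the board, sets player/AI roles and runs turns until the game ends.
; Rule and AI calls (Drop, Judge, Next, GetTurn) are defined outside these graphs.
; DropByPlayer records both human and AI moves, then either ends the game through UMG_Menu or triggers a delayed AI move.
; BP_Piece actors are matched by X/Y tags to place AI moves and spawn particles along the winning line.
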(event Custom|Init
  (Class|GobangFunction|Initialize)
  (CallFunction|ResetAllPieces)
  (Variables|Default|SetIsWon false))

(event Custom|SetMode
  (params (FirstPlayer :type Integer) (SecondPlayer :type Integer))
  (Variables|Default|SetFirstPlayer FirstPlayer)
  (bind _output_get (Variables|Default|SetSecondPlayer SecondPlayer))
  (Variables|Default|SetGameMode (- (+ _output_get (Variables|Default|GetFirstPlayer)) 1))
  (if (== (Variables|Default|GetFirstPlayer) 2)
    (CallFunction|DropbyAI)))

(event Custom|DropByPlayer
  (params (X :type Integer) (Y :type Integer))
  (Class|GobangFunction|Drop X Y)
  (Math|Integer|IncrementInt (Variables|Default|GetCntPieces)
    (:%20%20
      (bind _returnvalue (Class|GobangFunction|Judge))
      (if (Math|Conversions|ToBoolean(Integer) _returnvalue)
        (bind (_x1 _y1 _x2 _y2) (Class|GobangFunction|GetWinningPos))
        (CallFunction|ShowWinningPos _x1 _y1 _x2 _y2)
        (Variables|Default|SetIsWon true :!label _label)
        (bind _foundwidgets (Widget|GetAllWidgetsOfClass "/Game/Widgets/UMG_Menu.UMG_Menu_C" true))
        (Default|Won (Utilities|Array|Get(acopy) _foundwidgets))
        (else
          (bind _returnvalue_2 (Class|GobangFunction|GetTurn))
          (if (== _returnvalue_2 0)
            (goto _label)
            (else
              (bind _val (CallFunction|Who'sTurn))
              (if (== _val 2)
                (Utilities|FlowControl|Delay 1.0)
                (CallFunction|DropbyAI)))))))))

(event Custom|DropByAI
  (Math|Integer|IncrementInt (Variables|Default|GetCntPieces)
    (:%20%20
      (bind (_x _y) (Class|GobangFunction|Next))
      (bind _pieceref (CallFunction|FindPiece _x _y))
      (Default|DropbyAI _pieceref)
      (CallFunction|DropbyPlayer _x _y))))

(fn ConstructionScript)

(fn ShowWinningPos
  (params (X1 :type Integer) (Y1 :type Integer) (X2 :type Integer) (Y2 :type Integer))
  (LocalVariables|SetSignX (/ (- X2 X1) 4))
  (LocalVariables|SetSignY (/ (- Y2 Y1) 4))
  (for _index (range 0 4)
    (LocalVariables|SetIndex _index)
    (bind _outactors (Actor|GetAllActorsOfClass "/Game/Blueprints/BP_Piece.BP_Piece_C"))
    (bind _array_element (Utilities|Array|ForEachLoopwithBreak _outactors :!label _label)
      (:LoopBody
        (if (Utilities|Array|Identical (Variables|/Script/Engine.Actor|GetTags _array_element) (Utilities|Array|MakeArray (Utilities|String|StringToName (Utilities|String|ToString(Integer) (+ X1 (* (LocalVariables|GetSignX) (LocalVariables|GetIndex))))) (Utilities|String|StringToName (Utilities|String|ToString(Integer) (+ Y1 (* (LocalVariables|GetSignY) (LocalVariables|GetIndex)))))))
          (Effects|SpawnEmitteratLocation "/Game/Gomoku/Particles/P_vara1.P_vara1" (Transformation|GetActorLocation _array_element) (Transformation|GetActorRotation _array_element) "0.150000,0.150000,0.150000")
          (goto _label Break))))))

(fn ResetAllPieces
  (bind _outactors (Actor|GetAllActorsOfClass "/Game/Blueprints/BP_Piece.BP_Piece_C"))
  (for _array_element _outactors
    (Development|SetHiddeninGame (Variables|/Game/Blueprints/BP_Piece.BP_Piece_C|GetPiece _array_element) true false)
    (Rendering|Material|SetMaterial (Variables|/Game/Blueprints/BP_Piece.BP_Piece_C|GetPiece _array_element) 0 "/Engine/EngineMaterials/DefaultMaterial.DefaultMaterial")
    (Variables|/Game/Blueprints/BP_Piece.BP_Piece_C|SetIsDropped _array_element false))
  (return))

(fn Who'sTurn
  (bind _returnvalue (Class|GobangFunction|GetTurn))
  (if (or (and (== (Variables|Default|GetSecondPlayer) 1) (== _returnvalue 2)) (and (== _returnvalue 1) (== (Variables|Default|GetFirstPlayer) 1)))
    (return 1)
    (else
      (return 2))))

(fn FindPiece
  (params (X :type Integer) (Y :type Integer))
  (bind _outactors (Actor|GetAllActorsOfClass "/Game/Blueprints/BP_Piece.BP_Piece_C"))
  (bind _array_element (Utilities|Array|ForEachLoopwithBreak _outactors)
    (:LoopBody
      (if (Utilities|Array|Identical (Variables|/Script/Engine.Actor|GetTags _array_element) (Utilities|Array|MakeArray (Utilities|String|StringToName (Utilities|String|ToString(Integer) X)) (Utilities|String|StringToName (Utilities|String|ToString(Integer) Y))))
        (return _array_element)))))