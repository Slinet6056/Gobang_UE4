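; BP_Piece is one board point in a Gobang game, a hidden piece mesh that becomes a placed stone.
; Hover previews it in the current turn's black or white material when BP_GobangFunction allows a player move and the point is free.
; Release plays a sound, locks the piece and reports its coordinates, read from actor Tags, to BP_GobangFunction.
; DropByAI places it likewise, without reporting back.
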(event OnBeginCursorOver(Piece)
  (params (TouchedComponent :type Primitive%20Component%20Object%20Reference))
  (bind _candrop (Utilities|CanDrop))
  (if _candrop
    (CallFunction|ShowPiece)))

(event OnEndCursorOver(Piece)
  (params (TouchedComponent :type Primitive%20Component%20Object%20Reference))
  (if (not (Variables|Default|GetIsDropped))
    (CallFunction|HidePiece)))

(event OnReleased(Piece)
  (params (TouchedComponent :type Primitive%20Component%20Object%20Reference) (ButtonReleased :type Key%20Structure))
  (bind _candrop (Utilities|CanDrop))
  (if _candrop
    (CallFunction|DropbyPlayer)))

(fn ConstructionScript)

(fn GetTurn
  (bind _outactors (Actor|GetAllActorsOfClass "/Game/Blueprints/BP_GobangFunction.BP_GobangFunction_C"))
  (bind _returnvalue (Class|GobangFunction|GetTurn (Utilities|Array|Get(acopy) _outactors)))
  (return _returnvalue))

(fn ShowPiece
  (bind _piece (Variables|Default|GetPiece))
  (Development|SetHiddeninGame (Variables|Default|GetPiece) false false)
  (bind _turn (CallFunction|GetTurn))
  (switch int _turn
    (:1
      (Rendering|Material|SetMaterial _piece 0 "/Game/Puzzle/Meshes/BlackMaterial.BlackMaterial"))
    (:2
      (Rendering|Material|SetMaterial _piece 0 "/Game/Puzzle/Meshes/WhiteMaterial.WhiteMaterial")))
  (return))

(fn HidePiece
  (bind _piece (Variables|Default|GetPiece))
  (Development|SetHiddeninGame _piece true false)
  (Rendering|Material|SetMaterial _piece 0 "/Engine/EngineMaterials/DefaultMaterial.DefaultMaterial"))

(fn DropbyPlayer
  (bind (_x _y) (Utilities|GetPos))
  (Audio|SpawnSoundatLocation "/Game/Gomoku/Sound/落子_WAV_Cue.落子_WAV_Cue" (Transformation|GetActorLocation) "0, 0, 0" 1.0 1.0 0.0 0 0)
  (CallFunction|ShowPiece)
  (Variables|Default|SetIsDropped true)
  (bind _outactors (Actor|GetAllActorsOfClass "/Game/Blueprints/BP_GobangFunction.BP_GobangFunction_C"))
  (Default|DropbyPlayer (Utilities|Array|Get(acopy) _outactors) _x _y))

(fn DropbyAI
  (Audio|SpawnSoundatLocation "/Game/Gomoku/Sound/落子_WAV_Cue.落子_WAV_Cue" (Transformation|GetActorLocation) "0, 0, 0" 1.0 1.0 0.0 0 0)
  (CallFunction|ShowPiece)
  (Variables|Default|SetIsDropped true))